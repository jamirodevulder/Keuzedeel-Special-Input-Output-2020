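; Game mode Blueprint that runs a countdown timer for a game session.
; BeginPlay creates the Timer widget and adds it to the viewport.
; Tick passes through a one-second Delay, so TimeSec drops by one about once per second until GameDone is set.
; A following check on TimeSec being zero or above has no actions attached, so nothing here handles the timer running out.
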(event EventBeginPlay
  (bind _returnvalue (UserInterface|CreateWidget "/Game/timer.timer_C"))
  (UserInterface|Viewport|AddtoViewport _returnvalue 0))

(event EventTick
  (params (DeltaSeconds :type Float%20%28single-precision%29))
  (Utilities|FlowControl|Delay 1.0)
  (if (Variables|Default|GetGameDone)
    _
    (else
      (bind _output_get (Variables|Default|Settime%20sec (- (Variables|Default|Gettime%20sec) 1)))))
  (if (>= _output_get 0)
    _))

(fn ConstructionScript)